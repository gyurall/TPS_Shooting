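; Third-person shooter player Blueprint that connects the character to its HUD, game-over screen and physical hit reactions.
; BeginPlay creates the HUD widget for HP and grenade weapon-swap display, while game over shows the cursor and a game-over widget once.
; Tick stores control pitch and moves the actor with the spine bone while ragdolled.
; OnDamaged briefly simulates physics from spine_01 down, using a timeline to drive the blend weight.
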(event EventBeginPlay
  (bind _returnvalue (UserInterface|CreateWidget "/Game/Widget/UI_Screen.UI_Screen_C" (Game|GetPlayerController 0)))
  (bind _output_get (Variables|Default|SetuiScreen _returnvalue))
  (UserInterface|Viewport|AddtoViewport _output_get 0)
  (Utilities|FlowControl|Delay 0.05)
  (CallFunction|UIctrlHP)
  (Class|TPSPlayer|OnUsingGrenade false))

(event EventTick
  (params (DeltaSeconds :type Float%20%28single-precision%29))
  (Utilities|FlowControl|Sequence
    (:then_0
      (CallFunction|UpdatePitch))
    (:then_1
      (if (Variables|Default|GetisRagdoll)
        (Transformation|SetActorLocation (+ (Transformation|GetSocketLocation (Variables|Character|GetMesh) "spine_01") "0, 0,60.000000") false false)))))

(event EventOnUsingGrenade
  (params (isGrenade :type Boolean))
  (bind _uiscreen (Variables|Default|GetuiScreen))
  (Utilities|IsValid _uiscreen
    (:Is%20Valid
      (Variables|/Game/Widget/UI_Screen.UI_Screen_C|SetisGrenaded _uiscreen isGrenade)
      (Default|SwapWeapon _uiscreen))))

(event EventOnGameOver
  (bind _returnvalue (Game|GetPlayerController 0))
  (|CallParentFunction)
  (Utilities|FlowControl|DoOnce false
    (:Completed
      (Variables|/Script/Engine.PlayerController|SetbShowMouseCursor _returnvalue true)
      (bind _returnvalue_2 (UserInterface|CreateWidget "/Game/Widget/UI_GameOver.UI_GameOver_C" _returnvalue))
      (UserInterface|Viewport|AddtoViewport _returnvalue_2 0))))

(event EventOnDamaged
  (bind _returnvalue (Utilities|Name|MakeLiteralName "spine_01"))
  (bind _returnvalue_2 (Utilities|Name|MakeLiteralName "spine_01"))
  (Class|SkeletalMeshComponent|SetAllBodiesBelowSimulatePhysics (Variables|Character|GetMesh) _returnvalue true true)
  (Class|SkeletalMeshComponent|SetAllBodiesBelowPhysicsBlendWeight (Variables|Character|GetMesh) _returnvalue 1.0 false true)
  (bind _blendweight (Timeline|BlendWeight PlayFromStart)
    (:Update
      (Class|SkeletalMeshComponent|SetAllBodiesBelowPhysicsBlendWeight (Variables|Character|GetMesh) _returnvalue_2 _blendweight false true))
    (:Finished
      (Class|SkeletalMeshComponent|SetAllBodiesBelowSimulatePhysics (Variables|Character|GetMesh) _returnvalue_2 false true))))

(fn ConstructionScript)

(fn UIctrlHP
  (bind _uiscreen (Variables|Default|GetuiScreen))
  (Variables|/Game/Widget/UI_Screen.UI_Screen_C|SethpRatio _uiscreen (/ (Math|Conversions|ToFloat(Integer) (Variables|Default|Gethp)) (Math|Conversions|ToFloat(Integer) (Variables|Default|GetinitialHp))))
  (Variables|/Game/Widget/UI_Screen.UI_Screen_C|SethpString _uiscreen (Utilities|String|Append (Utilities|String|ToString(Integer) (Variables|Default|Gethp)) "/" (Utilities|String|ToString(Integer) (Variables|Default|GetinitialHp)))))

(fn UpdatePitch
  (Variables|Default|SetPitch (.pitch (Pawn|GetControlRotation :!class /Script/Engine.Pawn))))

(fn OnHitEven)